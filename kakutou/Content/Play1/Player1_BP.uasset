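; Player 1's character Blueprint, handling movement, camera look, jumping and attacks through Enhanced Input.
; On possession it casts the controller to PlayerController and adds the IMC_Player1 mapping context to the local player subsystem.
; WS and AD input move the character along the control rotation's yaw-only forward and right vectors, while turn and look-up drive controller yaw and pitch.
; Left, right and C-named mouse actions play attack, kick and Chapa montages on the mesh.
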(event `self.ReceivePossessed`
  (params (NewController :type "Controller Object Reference"))
  ;[1 1 1] 入力キーテーブルをコントローラーに割り当て
  (bind _asplayer_controller (cast `PlayerController` NewController))
  (message `EnhancedInputSubsystemInterface.AddMappingContext` (pcsubsystem `EnhancedInputLocalPlayerSubsystem` _asplayer_controller) "/Game/Play1/KeyEvent/IMC_Player1.IMC_Player1" 0 (struct)))

(event `EnhancedInput|/Game/Play1/KeyEvent/IMC_Jump`
  (params (ActionValue :type "Float (double-precision)") (ElapsedSeconds :type "Float (double-precision)") (TriggeredSeconds :type "Float (double-precision)") (InputAction :type "InputAction Object Reference" :default "/Game/Play1/KeyEvent/IMC_Jump.IMC_Jump"))
  (:`Triggered`
    (`self.Jump`)))

(event `EnhancedInput|/Game/Play1/KeyEvent/IMC_MouseL`
  (params (ActionValue :type Boolean) (ElapsedSeconds :type "Float (double-precision)") (TriggeredSeconds :type "Float (double-precision)") (InputAction :type "InputAction Object Reference" :default "/Game/Play1/KeyEvent/IMC_MouseL.IMC_MouseL"))
  (:`Triggered`
    (`|PlayMontage` (`self.Mesh`) "/Game/Play1/Animation/P1Attack_MTG.P1Attack_MTG")))

(event `EnhancedInput|/Game/Play1/KeyEvent/IMC_Turn`
  (params (ActionValue :type "Float (double-precision)") (ElapsedSeconds :type "Float (double-precision)") (TriggeredSeconds :type "Float (double-precision)") (InputAction :type "InputAction Object Reference" :default "/Game/Play1/KeyEvent/IMC_Turn.IMC_Turn"))
  ;[1 1 1] マウスでカメラアングルの切り替え
  (:`Triggered`
    (`self.AddControllerYawInput` ActionValue)))

(event `EnhancedInput|/Game/Play1/KeyEvent/IMC_LoockUp`
  (params (ActionValue :type "Float (double-precision)") (ElapsedSeconds :type "Float (double-precision)") (TriggeredSeconds :type "Float (double-precision)") (InputAction :type "InputAction Object Reference" :default "/Game/Play1/KeyEvent/IMC_LoockUp.IMC_LoockUp"))
  ;[1 1 1] マウスでカメラアングルの切り替え
  (:`Triggered`
    (`self.AddControllerPitchInput` ActionValue)))

(event `EnhancedInput|/Game/Play1/KeyEvent/IMC_MouseR`
  (params (ActionValue :type Boolean) (ElapsedSeconds :type "Float (double-precision)") (TriggeredSeconds :type "Float (double-precision)") (InputAction :type "InputAction Object Reference" :default "/Game/Play1/KeyEvent/IMC_MouseR.IMC_MouseR"))
  (:`Triggered`
    (`|PlayMontage` (`self.Mesh`) "/Game/Play1/Animation/P1Kick_Montage.P1Kick_Montage")))

(event `EnhancedInput|/Game/Play1/KeyEvent/IMC_WS`
  (params (ActionValue :type "Float (double-precision)") (ElapsedSeconds :type "Float (double-precision)") (TriggeredSeconds :type "Float (double-precision)") (InputAction :type "InputAction Object Reference" :default "/Game/Play1/KeyEvent/IMC_WS.IMC_WS"))
  (bind (_returnvalue_roll _returnvalue_pitch _returnvalue_yaw) (`KismetMathLibrary.BreakRotator` (`self.GetControlRotation`)))
  (:`Triggered`
    (`self.AddMovementInput` (`KismetMathLibrary.GetForwardVector` (`KismetMathLibrary.MakeRotator` 0.0 0.0 _returnvalue_yaw)) ActionValue)))

(event `EnhancedInput|/Game/Play1/KeyEvent/IMC_MouseC`
  (params (ActionValue :type Boolean) (ElapsedSeconds :type "Float (double-precision)") (TriggeredSeconds :type "Float (double-precision)") (InputAction :type "InputAction Object Reference" :default "/Game/Play1/KeyEvent/IMC_MouseC.IMC_MouseC"))
  (:`Triggered`
    (`|PlayMontage` (`self.Mesh`) "/Game/Play1/Animation/P1Chapa_Montage.P1Chapa_Montage")))

(event `EnhancedInput|/Game/Play1/KeyEvent/IMC_AD`
  (params (ActionValue :type "Float (double-precision)") (ElapsedSeconds :type "Float (double-precision)") (TriggeredSeconds :type "Float (double-precision)") (InputAction :type "InputAction Object Reference" :default "/Game/Play1/KeyEvent/IMC_AD.IMC_AD"))
  (bind (_returnvalue_roll _returnvalue_pitch _returnvalue_yaw) (`KismetMathLibrary.BreakRotator` (`self.GetControlRotation`)))
  (:`Triggered`
    (`self.AddMovementInput` (`KismetMathLibrary.GetRightVector` (`KismetMathLibrary.MakeRotator` 0.0 0.0 _returnvalue_yaw)) ActionValue)))

(fn `UserConstructionScript`)
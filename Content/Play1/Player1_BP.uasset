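; Player 1's playable character Blueprint, which adds its Enhanced Input mapping on possession and handles yaw-relative movement, jumping and three mouse-button attack montages.
; Attacks set an Attackeffect flag that blocks movement and jumping until Flagoff_Event clears it.
; Separate events toggle the axe hitbox collision and play a damage montage.
; The body-box overlap casts to Player2_BP and a box component but has no further effect yet.
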(event `self.ReceivePossessed`
  (params (NewController :type "Controller Object Reference"))
  ;[1 1 1] 入力キーテーブルをコントローラーに割り当て
  (bind _asplayer_controller (cast `PlayerController` NewController))
  (message `EnhancedInputSubsystemInterface.AddMappingContext` (pcsubsystem `EnhancedInputLocalPlayerSubsystem` _asplayer_controller) "/Game/Play1/KeyEvent/IMC_Player1.IMC_Player1" 0 (struct)))

(event `EnhancedInput|/Game/Play1/KeyEvent/IMC_Jump`
  (params (ActionValue :type "Float (double-precision)") (ElapsedSeconds :type "Float (double-precision)") (TriggeredSeconds :type "Float (double-precision)") (InputAction :type "InputAction Object Reference" :default "/Game/Play1/KeyEvent/IMC_Jump.IMC_Jump"))
  (:`Triggered`
    (if (not (`self.attackeffect`))
      (`self.Jump`))))

(event `EnhancedInput|/Game/Play1/KeyEvent/IMC_MouseL`
  (params (ActionValue :type Boolean) (ElapsedSeconds :type "Float (double-precision)") (TriggeredSeconds :type "Float (double-precision)") (InputAction :type "InputAction Object Reference" :default "/Game/Play1/KeyEvent/IMC_MouseL.IMC_MouseL"))
  (:`Triggered`
    (`|PlayMontage` (`self.Mesh`) "/Game/Play1/Animation/P1Attack_MTG.P1Attack_MTG"
      (:`then`
        (set `self.attackeffect` true :!label _label)))))

(event `カスタムイベント_0`
  (`|PlayMontage` (`self.Mesh`) "/Game/Play1/Animation/P1_damage.P1_damage"))

(event `EnhancedInput|/Game/Play1/KeyEvent/IMC_MouseR`
  (params (ActionValue :type Boolean) (ElapsedSeconds :type "Float (double-precision)") (TriggeredSeconds :type "Float (double-precision)") (InputAction :type "InputAction Object Reference" :default "/Game/Play1/KeyEvent/IMC_MouseR.IMC_MouseR"))
  (:`Triggered`
    (`|PlayMontage` (`self.Mesh`) "/Game/Play1/Animation/P1Kick_Montage.P1Kick_Montage"
      (:`then`
        (goto _label)))))

(event `EnhancedInput|/Game/Play1/KeyEvent/IMC_WS`
  (params (ActionValue :type "Float (double-precision)") (ElapsedSeconds :type "Float (double-precision)") (TriggeredSeconds :type "Float (double-precision)") (InputAction :type "InputAction Object Reference" :default "/Game/Play1/KeyEvent/IMC_WS.IMC_WS"))
  (bind (_returnvalue_roll _returnvalue_pitch _returnvalue_yaw) (`KismetMathLibrary.BreakRotator` (`self.GetControlRotation`)))
  (:`Triggered`
    (if (not (`self.attackeffect`))
      (`self.AddMovementInput` (`KismetMathLibrary.GetForwardVector` (`KismetMathLibrary.MakeRotator` 0.0 0.0 _returnvalue_yaw)) ActionValue))))

(event `EnhancedInput|/Game/Play1/KeyEvent/IMC_MouseC`
  (params (ActionValue :type Boolean) (ElapsedSeconds :type "Float (double-precision)") (TriggeredSeconds :type "Float (double-precision)") (InputAction :type "InputAction Object Reference" :default "/Game/Play1/KeyEvent/IMC_MouseC.IMC_MouseC"))
  (:`Triggered`
    (`|PlayMontage` (`self.Mesh`) "/Game/Play1/Animation/P1Chapa_Montage.P1Chapa_Montage"
      (:`then`
        (goto _label)))))

(event `P1 AxeCollision_ON`
  ;[1 1 1] 斧のあたり範囲のONかDFFにする
  (`PrimitiveComponent.SetCollisionEnabled` (`self.AX_Box`) "QueryAndPhysics"))

(event `P1 AxeCollision_OFF`
  ;[1 1 1] 斧のあたり範囲のONかDFFにする
  (`PrimitiveComponent.SetCollisionEnabled` (`self.AX_Box`) "NoCollision"))

(event `EnhancedInput|/Game/Play1/KeyEvent/IMC_AD`
  (params (ActionValue :type "Float (double-precision)") (ElapsedSeconds :type "Float (double-precision)") (TriggeredSeconds :type "Float (double-precision)") (InputAction :type "InputAction Object Reference" :default "/Game/Play1/KeyEvent/IMC_AD.IMC_AD"))
  (bind (_returnvalue_roll _returnvalue_pitch _returnvalue_yaw) (`KismetMathLibrary.BreakRotator` (`self.GetControlRotation`)))
  (:`Triggered`
    (if (not (`self.attackeffect`))
      (`self.AddMovementInput` (`KismetMathLibrary.GetRightVector` (`KismetMathLibrary.MakeRotator` 0.0 0.0 _returnvalue_yaw)) ActionValue))))

(event `Flagoff_Event`
  (set `self.attackeffect` false))

(event `OnComponentBeginOverlap_body_Box`
  (params (OverlappedComponent :type "PrimitiveComponent Object Reference") (OtherActor :type "Actor Object Reference") (OtherComp :type "PrimitiveComponent Object Reference") (OtherBodyIndex :type Integer) (bFromSweep :type Boolean) (SweepResult :type "HitResult Structure (by ref)"))
  (cast `/Game/Play2/Player2_BP` OtherActor)
  (bind _asbox_collision (cast `BoxComponent` OtherComp)))

(fn `UserConstructionScript`)
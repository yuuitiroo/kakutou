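; Player 2 character Blueprint with Enhanced Input movement, jumping and three melee attacks.
; On possession it adds the IMC_Player2 mapping context to the controller.
; Punch, hook and kick inputs play montages and immediately clear AttackOff, as does Attack_Off_Event; nothing here sets it true.
; Jump and control-yaw-relative movement run only while AttackOff is false.
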(event `self.ReceivePossessed`
  (params (NewController :type "Controller Object Reference"))
  ;[1 1 1] 入力キーテーブルをコントローラーに割り当て
  (bind _asplayer_controller (cast `PlayerController` NewController))
  (message `EnhancedInputSubsystemInterface.AddMappingContext` (pcsubsystem `EnhancedInputLocalPlayerSubsystem` _asplayer_controller) "/Game/Play2/KeyEvent/IMC_Player2.IMC_Player2" 0 (struct)))

(event `EnhancedInput|/Game/Play2/KeyEvent/IMC_MouseL2`
  (params (ActionValue :type Boolean) (ElapsedSeconds :type "Float (double-precision)") (TriggeredSeconds :type "Float (double-precision)") (InputAction :type "InputAction Object Reference" :default "/Game/Play2/KeyEvent/IMC_MouseL2.IMC_MouseL2"))
  (:`Triggered`
    (`|PlayMontage` (`self.Mesh`) "/Game/Play2/Animation/P2_punch_Montage.P2_punch_Montage"
      (:`then`
        (set `self.Attack_Off` false :!label _label)))))

(event `EnhancedInput|/Game/Play2/KeyEvent/IMC_Jump2`
  (params (ActionValue :type "Float (double-precision)") (ElapsedSeconds :type "Float (double-precision)") (TriggeredSeconds :type "Float (double-precision)") (InputAction :type "InputAction Object Reference" :default "/Game/Play2/KeyEvent/IMC_Jump2.IMC_Jump2"))
  (:`Triggered`
    (if (not (`self.Attack_Off`))
      (`self.Jump`))))

(event `EnhancedInput|/Game/Play2/KeyEvent/IMC_MouseR2`
  (params (ActionValue :type Boolean) (ElapsedSeconds :type "Float (double-precision)") (TriggeredSeconds :type "Float (double-precision)") (InputAction :type "InputAction Object Reference" :default "/Game/Play2/KeyEvent/IMC_MouseR2.IMC_MouseR2"))
  (:`Triggered`
    (`|PlayMontage` (`self.Mesh`) "/Game/Play2/Animation/P2_Hook_Punch_Montage.P2_Hook_Punch_Montage"
      (:`then`
        (goto _label)))))

(event `EnhancedInput|/Game/Play2/KeyEvent/IMC_MouseC2`
  (params (ActionValue :type Boolean) (ElapsedSeconds :type "Float (double-precision)") (TriggeredSeconds :type "Float (double-precision)") (InputAction :type "InputAction Object Reference" :default "/Game/Play2/KeyEvent/IMC_MouseC2.IMC_MouseC2"))
  (:`Triggered`
    (`|PlayMontage` (`self.Mesh`) "/Game/Play2/Animation/P2Kicking_Montage.P2Kicking_Montage"
      (:`then`
        (goto _label)))))

(event `EnhancedInput|/Game/Play2/KeyEvent/IMC_WS2`
  (params (ActionValue :type "Float (double-precision)") (ElapsedSeconds :type "Float (double-precision)") (TriggeredSeconds :type "Float (double-precision)") (InputAction :type "InputAction Object Reference" :default "/Game/Play2/KeyEvent/IMC_WS2.IMC_WS2"))
  (bind (_returnvalue_roll _returnvalue_pitch _returnvalue_yaw) (`KismetMathLibrary.BreakRotator` (`self.GetControlRotation`)))
  (:`Triggered`
    (if (not (`self.Attack_Off`))
      (`self.AddMovementInput` (`KismetMathLibrary.GetForwardVector` (`KismetMathLibrary.MakeRotator` 0.0 0.0 _returnvalue_yaw)) ActionValue))))

(event `EnhancedInput|/Game/Play2/KeyEvent/IMC_AD2`
  (params (ActionValue :type "Float (double-precision)") (ElapsedSeconds :type "Float (double-precision)") (TriggeredSeconds :type "Float (double-precision)") (InputAction :type "InputAction Object Reference" :default "/Game/Play2/KeyEvent/IMC_AD2.IMC_AD2"))
  (bind (_returnvalue_roll _returnvalue_pitch _returnvalue_yaw) (`KismetMathLibrary.BreakRotator` (`self.GetControlRotation`)))
  (:`Triggered`
    (if (not (`self.Attack_Off`))
      (`self.AddMovementInput` (`KismetMathLibrary.GetRightVector` (`KismetMathLibrary.MakeRotator` 0.0 0.0 _returnvalue_yaw)) ActionValue))))

(event `Attack_Off_Event`
  (set `self.Attack_Off` false))

(fn `UserConstructionScript`)